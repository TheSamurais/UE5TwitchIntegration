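; Runs a timed Twitch chat poll whose result recolors every BP_Ball.
; Starting a poll feeds WBP_TwitchPollOverlay and subscribes to chat through a re-arming async wait.
; Each chatter's first message matching an entry, lowercased, updates the tally and overlay.
; FinishPoll closes the stream and passes the winning index to the balls, though PollWinningCount never updates, so the last entry with votes wins.
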(event `WaitForChannelChatMessage`
  (if (`self.bIsPollRunning`)
    (bind (_result _error) (`ApiWaitForUserMessageSentEvent.WaitForUserMessageSentEvent` (`self.ChannelChatTwitchEventStream`))
      (:`Done`
        (`self.ProcessMessageForPoll` _result)
        (`self.WaitForChannelChatMessage`))
      (:`Error`
        (`KismetSystemLibrary.PrintString` _error true true (struct :`R` 1.0 :`A` 1.0) 10.0)))
    (else
      (`KismetSystemLibrary.PrintString` "Poll is not running!" true true (struct :`G` 0.66 :`B` 1.0 :`A` 1.0) 10.0))))

(event `StartPollFromWidget`
  (params (PollTimeout :type "Float (single-precision)") (PollEntries :type "Array of String") (PollName :type Text))
  (if (and (not (`KismetArrayLibrary.Array_IsEmpty` PollEntries)) (not (`self.bIsPollRunning`)))
    (set `self.PollTimeout` PollTimeout)
    (set `self.PollEntries` PollEntries)
    (set `self.PollName` PollName)
    (bind _foundwidgets (`WidgetBlueprintLibrary.GetAllWidgetsOfClass` "/Game/TwitchIntegration/UI/WBP_TwitchPollOverlay.WBP_TwitchPollOverlay_C"))
    (bind _output (`|GetArrayItem` _foundwidgets))
    (`/Engine/EditorBlueprintResources/StandardMacros.IsValid` _output
      (:`Is Valid`
        (`/Game/TwitchIntegration/UI/WBP_TwitchPollOverlay.StartPollCountdown` _output (`self.PollName`) (`self.PollTimeout`) (`self.PollEntries`))
        (`KismetSystemLibrary.PrintString` "Starting Poll" true true (struct :`G` 1.0 :`B` 0.451579 :`A` 1.0) 5.0 :!label _label)
        (`KismetArrayLibrary.Array_Clear` (`self.ChatterPollEntries`))
        (`BlueprintMapLibrary.Map_Clear` (`self.PollEntriesCount`))
        (for _array_element (`self.PollEntries`)
          (`BlueprintMapLibrary.Map_Add` (`self.PollEntriesCount`) _array_element))
        (set `self.bIsPollRunning` true)
        (bind _returnvalue (`KismetSystemLibrary.K2_SetTimerDelegate` (`|CreateDelegate` :!event `FinishPoll`) (`self.PollTimeout`)))
        (set `self.PollTimerEvent` _returnvalue)
        (bind (_result _error) (`ApiSubscribeToEventStream.SubscribeToEventStream` "ChannelChatMessage")
          (:`Done`
            (set `self.ChannelChatTwitchEventStream` _result)
            (`self.WaitForChannelChatMessage`))
          (:`Error`
            (`KismetSystemLibrary.PrintString` _error true true (struct :`R` 1.0 :`A` 1.0) 10.0)))))))

(event `StartPollEditorDEBUG`
  (goto _label))

(event `FinishPoll`
  (bind _pollentriescount (`self.PollEntriesCount`))
  (bind _error (`ApiCloseEventStream.CloseEventStream` (`self.ChannelChatTwitchEventStream`))
    (:`Done`
      (`KismetSystemLibrary.PrintString` "Ending Poll" true true (struct :`R` 1.0 :`G` 0.739149 :`A` 1.0) 5.0)
      (set `self.bIsPollRunning` false)
      (bind _keys (`BlueprintMapLibrary.Map_Keys` _pollentriescount))
      (bind _values (`BlueprintMapLibrary.Map_Values` _pollentriescount))
      (`KismetSystemLibrary.PrintString` (`KismetTextLibrary.Conv_TextToString` (`|FormatText` "{choice1}: {votes1} \n{choice2}: {votes2} \n{choice3}: {votes3}" (`|GetArrayItem` _keys) (`|GetArrayItem` _values) (`|GetArrayItem` _keys 1) (`|GetArrayItem` _values 1) (`|GetArrayItem` _keys 2) (`|GetArrayItem` _values 2))))
      (set `self.PollWinningCount` 0)
      (for (_array_element _array_index) _values
        (if (> _array_element (`self.PollWinningCount`))
          (set `self.PollWinningEntryIndex` _array_index)))
      (bind _outactors (`GameplayStatics.GetAllActorsOfClass` "/Game/TwitchIntegration/BP_Ball.BP_Ball_C"))
      (for _array_element_2 _outactors
        (`/Game/TwitchIntegration/BP_Ball.ChangeBallColor` _array_element_2 (`self.PollWinningEntryIndex`))))
    (:`Error`
      (`KismetSystemLibrary.PrintString` _error true true (struct :`R` 1.0 :`A` 1.0) 10.0))))

(fn `ProcessMessageForPoll`
  (params (MessageSentEvent :type "TwitchSDKUserMessageSentEvent Structure"))
  (bind (_broadcasteruserid _broadcasterusername _broadcasteruserlogin _chatteruserid _chatterusername _chatteruserlogin _messageid _text) (break `TwitchSDKUserMessageSentEvent` MessageSentEvent))
  (bind _returnvalue (`KismetStringLibrary.ToLower` _text))
  (bind (_value _returnvalue_2) (`BlueprintMapLibrary.Map_Find` (`self.PollEntriesCount`) _returnvalue))
  (`KismetSystemLibrary.PrintString` (`KismetTextLibrary.Conv_TextToString` (`|FormatText` "{chatter}: {msg}" _chatterusername _text)))
  (if (not (`KismetArrayLibrary.Array_Contains` (`self.ChatterPollEntries`) _chatteruserid))
    (if _returnvalue_2
      (`KismetArrayLibrary.Array_Add` (`self.ChatterPollEntries`) _chatteruserid)
      (`BlueprintMapLibrary.Map_Add` (`self.PollEntriesCount`) _returnvalue (+ _value 1))
      (bind _foundwidgets (`WidgetBlueprintLibrary.GetAllWidgetsOfClass` "/Game/TwitchIntegration/UI/WBP_TwitchPollOverlay.WBP_TwitchPollOverlay_C"))
      (`/Game/TwitchIntegration/UI/WBP_TwitchPollOverlay.UpdatePollVote` (`|GetArrayItem` _foundwidgets) (`KismetArrayLibrary.Array_Find` (`self.PollEntries`) _returnvalue))
      (return)
      (else
        (return)))
    (else
      (return))))

(fn `UserConstructionScript`)