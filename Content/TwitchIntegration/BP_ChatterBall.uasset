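; BP_ChatterBall is a Twitch integration ball actor that represents a chatter with a color and a name label.
; BeginPlay creates a dynamic instance of MI_Ball on the sphere, and events set its Color parameter and the name text.
; Each Tick moves the text render to a fixed world-space height above the sphere, so the label follows the ball's position.
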(event `UpdateBallColor`
  (params (Value :type "LinearColor Structure"))
  (`MaterialInstanceDynamic.SetVectorParameterValue` (`self.BallDynamicMaterialInstance`) "Color" Value))

(event `SetBallChatterInfo`
  (params (Color :type "LinearColor Structure") (ChatterName :type "Text (by ref)"))
  (`MaterialInstanceDynamic.SetVectorParameterValue` (`self.BallDynamicMaterialInstance`) "Color" Color)
  (`TextRenderComponent.K2_SetText` (`self.TextRender`) ChatterName))

(event `self.ReceiveBeginPlay`
  (`parent.ReceiveBeginPlay`)
  (bind _returnvalue (`PrimitiveComponent.CreateDynamicMaterialInstance` (`self.Sphere`) 0 "/Game/TwitchIntegration/MI_Ball.MI_Ball" "None"))
  (set `self.BallDynamicMaterialInstance` _returnvalue))

(event `self.ReceiveTick`
  (params (DeltaSeconds :type "Float (single-precision)"))
  (`parent.ReceiveTick` DeltaSeconds)
  (`SceneComponent.K2_SetWorldLocation` (`self.TextRender`) (`KismetMathLibrary.MakeVector` (.x (`SceneComponent.K2_GetComponentLocation` (`self.Sphere`))) (.y (`SceneComponent.K2_GetComponentLocation` (`self.Sphere`))) (+ (.z (`SceneComponent.K2_GetComponentLocation` (`self.Sphere`))) 100.0)) false false))

(fn `UserConstructionScript`)