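; BP_Ball is a Twitch integration ball actor with a recolorable mesh and a viewer poll for choosing its color.
; BeginPlay creates a dynamic material instance, whose Color parameter ChangeBallColor sets to red, green or blue by index.
; CreatePollForChangeBallColor opens a timed poll, waits for an update, prints each choice's votes, then unsubscribes.
; The poll result never calls ChangeBallColor, and a timer node is left unconnected.
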(event `ChangeBallColor`
  (params (EntryIndex :type Integer))
  (`MaterialInstanceDynamic.SetVectorParameterValue` (`self.BallDynMaterialInstance`) "Color" (select `int` EntryIndex :`0` (struct :`R` 1.0 :`A` 1.0) :`1` (struct :`G` 1.0 :`A` 1.0) :`2` (struct :`B` 1.0 :`A` 1.0) :!type "LinearColor Structure")))

(event `self.ReceiveBeginPlay`
  (`parent.ReceiveBeginPlay`)
  (bind _returnvalue (`PrimitiveComponent.CreateDynamicMaterialInstance` (`self.BallMesh`) 0 "/Game/TwitchIntegration/MI_Ball.MI_Ball" "None"))
  (set `self.BallDynMaterialInstance` _returnvalue))

(event `CreatePollForChangeBallColor`
  (`KismetSystemLibrary.PrintString` "Creating poll")
  (bind (_result _error) (`ApiCreatePoll.CreatePoll` "To what color change ball to?" (`|MakeArray` "Red" "Blue" "Green") 20)
    (:`Done`
      (bind ((`Id` _id)) (break `TwitchSDKPollInfo` _result))
      (bind (_result_2 _error_2) (`ApiWaitForPollUpdate.WaitForPollUpdate` _id)
        (:`Done`
          (for _array_element (`.Choices` (break `TwitchSDKPollInfo` _result_2))
            (bind ((`Id` _id_2) (`Title` _title) (`Votes` _votes)) (break `TwitchSDKPollChoiceInfo` _array_element))
            (`KismetSystemLibrary.PrintString` (`KismetTextLibrary.Conv_TextToString` (`|FormatText` "ID: {id},  Title: {title},  no votes: {no}" _id_2 _title _votes))))
          (`ApiUnsubscribeFromPoll.UnsubscribeFromPoll` _id))
        (:`Error`
          (`KismetSystemLibrary.PrintString` _error_2 true true (struct :`R` 1.0 :`G` 0.019608 :`A` 1.0) 3.0))))
    (:`Error`
      (`KismetSystemLibrary.PrintString` _error true true (struct :`R` 1.0 :`G` 0.019608 :`A` 1.0) 3.0))))

(fn `UserConstructionScript`)